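; Ledge actor that defines a polyline through a LedgePoints array, stored as offsets from its CollisionComponent.
; On BeginPlay it caches the collision component's world location in Position.
; Every Tick it draws red debug lines between consecutive points at the component's current location, visualizing the ledge path.
; The file holds no grab or climb logic, and the construction script is empty.
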(event EventTick
  (params (DeltaSeconds :type Float%20%28single-precision%29))
  (bind _ledge_points (Variables|Default|GetLedge%20points))
  (bind _collisioncomponent (Variables|Default|GetCollisionComponent))
  (bind _returnvalue (Transformation|GetWorldLocation _collisioncomponent))
  (for _index (range 1 (- (Utilities|Array|Length (Variables|Default|GetLedge%20points)) 1))
    (Rendering|Debug|DrawDebugLine (+ _returnvalue (Utilities|Array|Get(acopy) _ledge_points (- _index 1))) (+ _returnvalue (Utilities|Array|Get(acopy) _ledge_points _index)) "(R=1.000000,G=0.000000,B=0.058993,A=1.000000)" 1.0 5.0)))

(event EventBeginPlay
  (Variables|Default|SetPosition (Transformation|GetWorldLocation (Variables|Default|GetCollisionComponent))))

(fn ConstructionScript)