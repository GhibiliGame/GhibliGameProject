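; Buddy AI character that follows the player, changing into a mist form when left too far behind.
; Tick moves it by SimpleMoveToLocation, or lerps a collisionless sphere "mist" toward the player until within minimum distance, where it reforms and stops.
; F toggles StopMove through a FlipFlop.
; While stopped or near the player, Tick also runs a debug-drawn camera line trace and spawns a NewBlueprint actor at the hit location every frame.
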(event EventTick
  (params (DeltaSeconds :type Float%20%28single-precision%29))
  (bind _returnvalue (Game|GetPlayerCharacter 0))
  (bind _returnvalue_2 (Transformation|GetActorLocation))
  (bind _returnvalue_3 (Game|GetPlayerCameraManager 0))
  (bind _ismist (Variables|Default|GetisMist))
  (bind _returnvalue_4 (Transformation|GetActorLocation _returnvalue))
  (bind _transformcomponent (Variables|/Script/Engine.PlayerCameraManager|GetTransformComponent _returnvalue_3))
  (if (Variables|Default|GetstopMove)
    (AI|Navigation|StopMovement (Pawn|GetController))
    (bind _outhit (Collision|LineTraceByChannel (Transformation|GetWorldLocation _transformcomponent) (* (Math|Vector|GetForwardVector _transformcomponent) 5e+03) "TraceTypeQuery1" false (Utilities|Array|MakeArray (Game|GetPlayerCharacter 0)) "Persistent" :!label _label))
    (Game|SpawnActorfromClass "/Game/GhibliGame/BluePrints/NewBlueprint.NewBlueprint_C" (Math|Conversions|ToTransform(Vector) (.location _outhit)) "Undefined" 0 0)
    (elif (and (not (Variables|Default|GetisMist)) (> (Math|Vector|Distance(Vector) (.location (Transformation|GetActorTransform (Game|GetPlayerCharacter 0))) (.location (Transformation|GetActorTransform))) (Variables|Default|GetmaxMistDistFromPlayer)))
      (CallFunction|StartMistForm)
      (elif (< (Math|Vector|Distance(Vector) _returnvalue_2 (Transformation|GetActorLocation (Game|GetPlayerCharacter 0))) (Variables|Default|GetminDistFromPlayer))
        (if _ismist
          (CallFunction|EndMistForm))
        (AI|Navigation|StopMovement (Pawn|GetController))
        (Development|PrintString (Utilities|String|ToString(Vector) _returnvalue_2))
        (goto _label)
        (elif _ismist
          (Transformation|SetActorLocation (Math|Vector|Lerp(Vector) (Transformation|GetActorLocation) _returnvalue_4 0.05) false false)
          (else
            (AI|Navigation|SimpleMovetoLocation (Pawn|GetController) _returnvalue_4)))))))

(event EventBeginPlay)

(event Input|KeyboardEvents|F
  (params (Key :type Key%20Structure :default "None"))
  (:Pressed
    (Utilities|FlowControl|FlipFlop
      (:A
        (Variables|Default|SetstopMove false)
        (AI|Navigation|StopMovement (Pawn|GetController)))
      (:B
        (Variables|Default|SetstopMove true)))))

(fn ConstructionScript)

(fn StartMistForm
  (Collision|SetCollisionEnabled (Variables|Character|GetMesh) "NoCollision")
  (Collision|SetCollisionEnabled (Variables|Collision|GetCapsuleComponent) "NoCollision")
  (Rendering|SetVisibility (Variables|Character|GetMesh) false false)
  (Rendering|SetVisibility (Variables|Components|GetSphere) true false)
  (Variables|Default|SetisMist true))

(fn EndMistForm
  (Collision|SetCollisionEnabled (Variables|Character|GetMesh) "QueryAndPhysics")
  (Collision|SetCollisionEnabled (Variables|Collision|GetCapsuleComponent) "QueryAndPhysics")
  (Rendering|SetVisibility (Variables|Character|GetMesh) true false)
  (Rendering|SetVisibility (Variables|Components|GetSphere) false false)
  (Variables|Default|SetisMist false))