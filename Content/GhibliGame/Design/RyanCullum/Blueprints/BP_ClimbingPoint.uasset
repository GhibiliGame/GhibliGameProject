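; BP_ClimbingPoint is a placeable climbing point with flags marking it as the start or end of a climb.
; When the ThirdPersonGhibli_RyanCopy character overlaps its Box, a start point registers itself as that character's current climb point.
; The construction script shows or hides the Box and EndClimb components to match the start and end flags.
; Only visibility is toggled, and the end flag drives no other logic here.
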(event OnComponentBeginOverlap(Box)
  (params (OverlappedComponent :type Primitive%20Component%20Object%20Reference) (OtherActor :type Actor%20Object%20Reference) (OtherComp :type Primitive%20Component%20Object%20Reference) (OtherBodyIndex :type Integer) (bFromSweep :type Boolean) (SweepResult :type Hit%20Result%20Structure%20%28by%20ref%29))
  (bind _asthird_person_ghibli_ryan_copy (Utilities|Casting|CastToThirdPersonGhibli_RyanCopy OtherActor))
  (if (Variables|Default|GetIsClimbStart)
    (Default|SetCurrentClimbPoint _asthird_person_ghibli_ryan_copy self)))

(event EventBeginPlay)

(event Collision|EventActorBeginOverlap
  (params (OtherActor :type Actor%20Object%20Reference)))

(event EventTick
  (params (DeltaSeconds :type Float%20%28single-precision%29)))

(fn ConstructionScript
  (if (Variables|Default|GetIsClimbEnd)
    (Rendering|SetVisibility (Variables|Default|GetEndClimb) true false)
    (else
      (Rendering|SetVisibility (Variables|Default|GetEndClimb) false false)))
  (if (Variables|Default|GetIsClimbStart)
    (Rendering|SetVisibility (Variables|Default|GetBox) true false)
    (else
      (Rendering|SetVisibility (Variables|Default|GetBox) false false))))