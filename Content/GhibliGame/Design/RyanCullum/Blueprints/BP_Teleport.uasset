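; BP_Teleport is a teleport point that offers its Cube's location as a destination to the player character.
; Box overlap sets CanTeleport and TeleportLocation on ThirdPersonGhibli_RyanCopy, and leaving clears CanTeleport.
; It also enables input for player 0, teleporting its Player reference to the Cube with the Arrow's rotation on Interact if CanClimb is true.
; Neither CanClimb nor Player is set in this graph.
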(event OnComponentBeginOverlap(Box)
  (params (OverlappedComponent :type Primitive%20Component%20Object%20Reference) (OtherActor :type Actor%20Object%20Reference) (OtherComp :type Primitive%20Component%20Object%20Reference) (OtherBodyIndex :type Integer) (bFromSweep :type Boolean) (SweepResult :type Hit%20Result%20Structure%20%28by%20ref%29))
  (bind _asthird_person_ghibli_ryan_copy (Utilities|Casting|CastToThirdPersonGhibli_RyanCopy OtherActor))
  (Variables|/Game/GhibliGame/Design/RyanCullum/Blueprints/ThirdPersonGhibli_RyanCopy.ThirdPersonGhibli_RyanCopy_C|SetCanTeleport _asthird_person_ghibli_ryan_copy true)
  (Variables|/Game/GhibliGame/Design/RyanCullum/Blueprints/ThirdPersonGhibli_RyanCopy.ThirdPersonGhibli_RyanCopy_C|SetTeleportLocation _asthird_person_ghibli_ryan_copy (Transformation|GetWorldLocation (Variables|Default|GetCube))))

(event OnComponentEndOverlap(Box)
  (params (OverlappedComponent :type Primitive%20Component%20Object%20Reference) (OtherActor :type Actor%20Object%20Reference) (OtherComp :type Primitive%20Component%20Object%20Reference) (OtherBodyIndex :type Integer))
  (bind _asthird_person_ghibli_ryan_copy (Utilities|Casting|CastToThirdPersonGhibli_RyanCopy OtherActor))
  (Variables|/Game/GhibliGame/Design/RyanCullum/Blueprints/ThirdPersonGhibli_RyanCopy.ThirdPersonGhibli_RyanCopy_C|SetCanTeleport _asthird_person_ghibli_ryan_copy false))

(event EventBeginPlay
  (Input|EnableInput (Game|GetPlayerController 0)))

(event Collision|EventActorBeginOverlap
  (params (OtherActor :type Actor%20Object%20Reference)))

(event EventTick
  (params (DeltaSeconds :type Float%20%28single-precision%29)))

(event Input|ActionEvents|InputActionInteract
  (params (Key :type Key%20Structure :default "None"))
  (:Pressed
    (if (Variables|Default|GetCanClimb)
      (Transformation|Teleport (Variables|Default|GetPlayer) (Transformation|GetWorldLocation (Variables|Default|GetCube)) (Transformation|GetWorldRotation (Variables|Default|GetArrow))))))

(fn ConstructionScript)